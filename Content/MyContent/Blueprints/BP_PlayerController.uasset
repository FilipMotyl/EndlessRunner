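; BP_PlayerController is a player controller that sets up the HUD and spawns the player's chosen character when play begins.
; On BeginPlay it creates BP_HUD_WB, adds it to the viewport and keeps a reference to it.
; It then spawns the SelectedCharacter class stored in the Main_GI game instance at the first PlayerStart found and possesses it.
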(event `self.ReceiveBeginPlay`
  (bind _returnvalue (`|CreateWidget` "/Game/MyContent/UI/BP_HUD_WB.BP_HUD_WB_C"))
  (`UserWidget.AddToViewport` _returnvalue 0)
  (set `self.HUDRef` _returnvalue)
  (bind _outactors (`GameplayStatics.GetAllActorsOfClass` "/Script/Engine.PlayerStart"))
  (bind _returnvalue_2 (`|SpawnActorFromClass` (`/Game/MyContent/Blueprints/Main_GI.SelectedCharacter` (cast `/Game/MyContent/Blueprints/Main_GI` (`GameplayStatics.GetGameInstance`) :!pure true)) (`self.GetTransform` (`|GetArrayItem` _outactors)) "Undefined" "OverrideRootScale" null null))
  (`self.Possess` _returnvalue_2))

(fn `UserConstructionScript`)