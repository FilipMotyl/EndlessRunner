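; BP_Character is a three-lane runner character that switches lanes, jumps and ends the game on hitting an obstacle.
; A and D step the lane side stored in BP_GameState and set a target Y, which Tick approaches at constant speed with a swept move, pinning X.
; Space drives jumping and a Jumping flag.
; The first Obstacle_Base hit shows the BP_EndScreen widget and mouse cursor.
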(event `Key|A`
  (params (Key :type "Key Structure"))
  (bind _leftlocation (`/Game/MyContent/Blueprints/Game/BP_GameState.LeftLocation` (`self.GameStateRef`)))
  ;[1 1 1] Move Left
  (:`Pressed`
    (set `self.TargetYLocation` (select `/Game/MyContent/Blueprints/Enums/ERoadSide` (`/Game/MyContent/Blueprints/Game/BP_GameState.Side` (`self.GameStateRef`)) :`NewEnumerator0` _leftlocation :`NewEnumerator1` _leftlocation :`NewEnumerator2` (`/Game/MyContent/Blueprints/Game/BP_GameState.MiddleLocation` (`self.GameStateRef`))))
    (set `/Game/MyContent/Blueprints/Game/BP_GameState.Side` (select `/Game/MyContent/Blueprints/Enums/ERoadSide` (`/Game/MyContent/Blueprints/Game/BP_GameState.Side` (`self.GameStateRef`)) :`NewEnumerator0` "NewEnumerator1" :`NewEnumerator1` "NewEnumerator1" :`NewEnumerator2` "NewEnumerator0" :!type "/Game/MyContent/Blueprints/Enums/ERoadSide Enum") (`self.GameStateRef`))))

(event `self.ReceiveBeginPlay`
  (bind _asbp_game_state (cast `/Game/MyContent/Blueprints/Game/BP_GameState` (`GameplayStatics.GetGameState`)))
  (set `self.GameStateRef` _asbp_game_state))

(event `Key|D`
  (params (Key :type "Key Structure"))
  (bind _rightlocation (`/Game/MyContent/Blueprints/Game/BP_GameState.RightLocation` (`self.GameStateRef`)))
  ;[1 1 1] Move Right
  (:`Pressed`
    (set `self.TargetYLocation` (select `/Game/MyContent/Blueprints/Enums/ERoadSide` (`/Game/MyContent/Blueprints/Game/BP_GameState.Side` (`self.GameStateRef`)) :`NewEnumerator0` _rightlocation :`NewEnumerator1` (`/Game/MyContent/Blueprints/Game/BP_GameState.MiddleLocation` (`self.GameStateRef`)) :`NewEnumerator2` _rightlocation))
    (set `/Game/MyContent/Blueprints/Game/BP_GameState.Side` (select `/Game/MyContent/Blueprints/Enums/ERoadSide` (`/Game/MyContent/Blueprints/Game/BP_GameState.Side` (`self.GameStateRef`)) :`NewEnumerator0` "NewEnumerator2" :`NewEnumerator1` "NewEnumerator0" :`NewEnumerator2` "NewEnumerator2" :!type "/Game/MyContent/Blueprints/Enums/ERoadSide Enum") (`self.GameStateRef`))))

(event `self.ReceiveTick`
  (params (DeltaSeconds :type "Float (single-precision)"))
  (bind (_returnvalue_x _returnvalue_y) (`KismetMathLibrary.BreakVector` (`self.K2_GetActorLocation`)))
  (bind (_returnvalue_x_2 _returnvalue_y_2 _returnvalue_z) (`KismetMathLibrary.BreakVector` (`self.K2_GetActorLocation`)))
  (`self.K2_SetActorLocation` (`KismetMathLibrary.MakeVector` 130.0 (`KismetMathLibrary.FInterpTo_Constant` _returnvalue_y (`self.TargetYLocation`) DeltaSeconds (`self.SidewaysSpeed`)) _returnvalue_z) true))

(event `Key|SpaceBar`
  (params (Key :type "Key Structure"))
  (:`Pressed`
    (`self.Jump`)
    (set `self.Jumping` true))
  (:`Released`
    (`self.StopJumping`)
    (set `self.Jumping` false)))

(event `self.ReceiveHit`
  (params (MyComp :type "PrimitiveComponent Object Reference") (Other :type "Actor Object Reference") (OtherComp :type "PrimitiveComponent Object Reference") (bSelfMoved :type Boolean) (HitLocation :type "Vector Structure") (HitNormal :type "Vector Structure") (NormalImpulse :type "Vector Structure") (Hit :type "HitResult Structure (by ref)"))
  (cast `/Game/MyContent/Blueprints/Game/Course/Obstacles/Obstacle_Base` Other)
  (`/Engine/EditorBlueprintResources/StandardMacros.DoOnce` false
    (:`Completed`
      (bind _returnvalue (`|CreateWidget` "/Game/MyContent/UI/BP_EndScreen.BP_EndScreen_C"))
      (`UserWidget.AddToViewport` _returnvalue 0)
      (set `PlayerController.bShowMouseCursor` true (`GameplayStatics.GetPlayerController` 0)))))

(fn `UserConstructionScript`)